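; Enemy melee AI unit that advances on a nexus destination and attacks pawns tagged "Friend".
; Tick drives the move to the nexus until PawnSensing spots any pawn, and sighted Friends are chased with AIMoveTo.
; On arrival it plays an attack montage and damages Friends found by a sphere overlap.
; It destroys itself at zero health, feeding a health widget shown while the first-person character overlaps its Sphere.
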(event OnSeePawn(PawnSensing)
  (params (Pawn :type Pawn%20Object%20Reference))
  (Variables|Default|Set적이%20%20보이는가? true)
  (if (Actor|ActorHasTag Pawn "Friend")
    (CallFunction|보이는적따라가기 Pawn)))

(event OnComponentBeginOverlap(Sphere)
  (params (OverlappedComponent :type Primitive%20Component%20Object%20Reference) (OtherActor :type Actor%20Object%20Reference) (OtherComp :type Primitive%20Component%20Object%20Reference) (OtherBodyIndex :type Integer) (bFromSweep :type Boolean) (SweepResult :type Hit%20Result%20Structure%20%28by%20ref%29))
  (Utilities|Casting|CastToBP_FirstPersonCharacter OtherActor)
  (Rendering|SetVisibility (Variables|Default|GetWidget) true false))

(event OnComponentEndOverlap(Sphere)
  (params (OverlappedComponent :type Primitive%20Component%20Object%20Reference) (OtherActor :type Actor%20Object%20Reference) (OtherComp :type Primitive%20Component%20Object%20Reference) (OtherBodyIndex :type Integer))
  (Utilities|Casting|CastToBP_FirstPersonCharacter OtherActor)
  (Rendering|SetVisibility (Variables|Default|GetWidget) false false))

(event Custom|보이는%20적%20따라가기
  (params (NewParam :type Actor%20Object%20Reference))
  (Variables|Default|Set공격%20가능? true)
  (if (Variables|Default|Get적이%20%20보이는가?)
    (AI|AIMoveTo self "0, 0, 0" NewParam 7e+01 false
      (:OnSuccess
        (if (Variables|Default|Get공격%20가능?)
          (bind _returnvalue (Animation|PlayAnimMontage "/Game/FlexibleCombatSystem/Montages/M_2H_AttackA.M_2H_AttackA" 1.0 "None"))
          (bind _outactors (Collision|SphereOverlapActors (Transformation|GetWorldLocation (Variables|Default|GetArrow1)) 1e+02 (Variables|Default|GetObject%20Types) 0))
          (bind _array_element (Utilities|Array|ForEachLoopwithBreak _outactors)
            (:LoopBody
              (if (Actor|ActorHasTag _array_element "Friend")
                (Game|Damage|ApplyDamage _array_element 1e+01 0 0)))
            (:Completed
              (Utilities|FlowControl|Delay _returnvalue)
              (Variables|Default|Set공격%20가능? false)
              (Variables|Default|Set적이%20%20보이는가? false))))))
    (else
      (Variables|Default|Set적이%20%20보이는가? false))))

(event EventBeginPlay
  (Variables|Default|SetHealth (Variables|Default|GetMaxHealth))
  (bind _asai_health_widget (Utilities|Casting|CastToAI_HealthWidget (UserInterface|GetUserWidgetObject (Variables|Default|GetWidget))))
  (Variables|Default|SetHealthWidgetREF _asai_health_widget))

(event EventTick
  (params (DeltaSeconds :type Float%20%28single-precision%29))
  (if (not (Variables|Default|Get적이%20%20보이는가?))
    (AI|AIMoveTo self (Variables|Default|GetnexuxDst) 0 5.0 false
      (:OnSuccess
        (Variables|Default|Set적이%20%20보이는가? false)))))

(event Game|Damage|EventAnyDamage
  (params (Damage :type Float%20%28single-precision%29) (DamageType :type Damage%20Type%20Object%20Reference) (InstigatedBy :type Controller%20Object%20Reference) (DamageCauser :type Actor%20Object%20Reference))
  (bind _output_get (Variables|Default|SetHealth (Math|Float|Clamp(Float) (- (Variables|Default|GetHealth) Damage) 0.0 (Variables|Default|GetMaxHealth))))
  (Variables|/Game/widgets/AI_HealthWidget.AI_HealthWidget_C|SetHealth (Variables|Default|GetHealthWidgetREF) _output_get)
  (if (== (Variables|Default|GetHealth) 0.0)
    (Actor|DestroyActor)))

(fn ConstructionScript)