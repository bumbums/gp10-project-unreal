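; Close-range enemy AI that chases the player on sight, plays a melee attack montage and is destroyed at zero health.
; PawnSensing sets a seen flag and starts AIMoveTo toward the player; Tick halts movement until that flag is set.
; Damage comes from the Hit event on any collided actor, independent of the montage.
; AnyDamage updates a health widget, shown only while the first-person character overlaps its sphere.
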(event OnSeePawn(PawnSensing)
  (params (Pawn :type Pawn%20Object%20Reference))
  (Variables|Default|Set플레이어가%20보이는가? true)
  (CallFunction|플레이어따라가기))

(event OnComponentBeginOverlap(Sphere)
  (params (OverlappedComponent :type Primitive%20Component%20Object%20Reference) (OtherActor :type Actor%20Object%20Reference) (OtherComp :type Primitive%20Component%20Object%20Reference) (OtherBodyIndex :type Integer) (bFromSweep :type Boolean) (SweepResult :type Hit%20Result%20Structure%20%28by%20ref%29))
  (Utilities|Casting|CastToBP_FirstPersonCharacter OtherActor)
  (Rendering|SetVisibility (Variables|Default|GetWidget) true false))

(event OnComponentEndOverlap(Sphere)
  (params (OverlappedComponent :type Primitive%20Component%20Object%20Reference) (OtherActor :type Actor%20Object%20Reference) (OtherComp :type Primitive%20Component%20Object%20Reference) (OtherBodyIndex :type Integer))
  (Utilities|Casting|CastToBP_FirstPersonCharacter OtherActor)
  (Rendering|SetVisibility (Variables|Default|GetWidget) false false))

(event Custom|플레이어%20따라가기
  (Variables|Default|Set공격%20가능? true)
  (if (Variables|Default|Get플레이어가%20보이는가?)
    (AI|AIMoveTo self "0, 0, 0" (Game|GetPlayerCharacter 0) 7e+01 false
      (:OnSuccess
        (if (Variables|Default|Get공격%20가능?)
          (Variables|Default|Set공격%20가능? true)
          (bind _returnvalue (Animation|PlayAnimMontage "/Game/FlexibleCombatSystem/Montages/M_2H_AttackA.M_2H_AttackA" 1.0 "None"))
          (Utilities|FlowControl|Delay _returnvalue)
          (Variables|Default|Set공격%20가능? false))))
    (else
      (Variables|Default|Set플레이어가%20보이는가? false))))

(event Collision|EventHit
  (params (MyComp :type Primitive%20Component%20Object%20Reference) (Other :type Actor%20Object%20Reference) (OtherComp :type Primitive%20Component%20Object%20Reference) (bSelfMoved :type Boolean) (HitLocation :type Vector :default "0, 0, 0") (HitNormal :type Vector :default "0, 0, 0") (NormalImpulse :type Vector :default "0, 0, 0") (Hit :type Hit%20Result%20Structure%20%28by%20ref%29))
  (Game|Damage|ApplyDamage Other 1e+01 0 0 "/Script/Engine.DamageType"))

(event EventBeginPlay
  (Variables|Default|SetHealth (Variables|Default|GetMaxHealth))
  (bind _asai_health_widget (Utilities|Casting|CastToAI_HealthWidget (UserInterface|GetUserWidgetObject (Variables|Default|GetWidget))))
  (Variables|Default|SetHealthWidgetREF _asai_health_widget))

(event EventTick
  (params (DeltaSeconds :type Float%20%28single-precision%29))
  (if (not (Variables|Default|Get플레이어가%20보이는가?))
    (Components|Movement|StopMovementImmediately (Variables|Character|GetCharacterMovement))))

(event Game|Damage|EventAnyDamage
  (params (Damage :type Float%20%28single-precision%29) (DamageType :type Damage%20Type%20Object%20Reference) (InstigatedBy :type Controller%20Object%20Reference) (DamageCauser :type Actor%20Object%20Reference))
  (bind _output_get (Variables|Default|SetHealth (Math|Float|Clamp(Float) (- (Variables|Default|GetHealth) Damage) 0.0 (Variables|Default|GetMaxHealth))))
  (Variables|/Game/widgets/AI_HealthWidget.AI_HealthWidget_C|SetHealth (Variables|Default|GetHealthWidgetREF) _output_get)
  (if (== (Variables|Default|GetHealth) 0.0)
    (Actor|DestroyActor)))

(fn ConstructionScript)