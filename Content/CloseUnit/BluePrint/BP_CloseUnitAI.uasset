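; BP_CloseUnitAI is a close-range AI unit that chases the player on sight and plays an attack montage on arrival.
; PawnSensing sets a visibility flag and calls the follow event, which re-arms attacking and runs AI MoveTo toward the player.
; A successful move triggers the montage once per arming, with no damage logic here.
; Tick halts movement until the first sighting, since the flag never resets afterward.
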(event OnSeePawn(PawnSensing)
  (params (Pawn :type Pawn%20Object%20Reference))
  (Variables|Default|Set플레이어가%20보이는가? true)
  (CallFunction|플레이어따라가기))

(event Custom|플레이어%20따라가기
  (Variables|Default|Set공격%20가능? true)
  (if (Variables|Default|Get플레이어가%20보이는가?)
    (AI|AIMoveTo self "0, 0, 0" (Game|GetPlayerCharacter 0) 7e+01 false
      (:OnSuccess
        (if (Variables|Default|Get공격%20가능?)
          (Variables|Default|Set공격%20가능? false)
          (bind _returnvalue (Animation|PlayAnimMontage "/Game/FirstPersonArms/Animations/FirstPersonFire_Montage.FirstPersonFire_Montage" 1.0 "None"))
          (Utilities|FlowControl|Delay _returnvalue)
          (Variables|Default|Set공격%20가능? false))))
    (else
      (Variables|Default|Set플레이어가%20보이는가? false))))

(event EventBeginPlay)

(event Collision|EventActorBeginOverlap
  (params (OtherActor :type Actor%20Object%20Reference)))

(event EventTick
  (params (DeltaSeconds :type Float%20%28single-precision%29))
  (if (not (Variables|Default|Get플레이어가%20보이는가?))
    (Components|Movement|StopMovementImmediately (Variables|Character|GetCharacterMovement))))

(fn ConstructionScript)