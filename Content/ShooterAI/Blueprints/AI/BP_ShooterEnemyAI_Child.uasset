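; Child shooter enemy AI that adds a proximity-shown health widget and its own weapon loadouts.
; BeginPlay sets EnemyHP and caches the health widget, while damage reduces a separate 현재체력 (current health) variable, clamped to its maximum.
; A sphere overlap shows the widget only while BP_FirstPersonCharacter is inside.
; WeaponSetup extends the parent, switching on weapon type to configure mesh, transform, combat stats and reload for assault rifle, machine gun or sniper.
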(event OnComponentBeginOverlap(Sphere_0)
  (params (OverlappedComponent :type Primitive%20Component%20Object%20Reference) (OtherActor :type Actor%20Object%20Reference) (OtherComp :type Primitive%20Component%20Object%20Reference) (OtherBodyIndex :type Integer) (bFromSweep :type Boolean) (SweepResult :type Hit%20Result%20Structure%20%28by%20ref%29))
  (Utilities|Casting|CastToBP_FirstPersonCharacter OtherActor)
  (Rendering|SetVisibility (Variables|Default|GetWidget) true false))

(event OnComponentEndOverlap(Sphere_0)
  (params (OverlappedComponent :type Primitive%20Component%20Object%20Reference) (OtherActor :type Actor%20Object%20Reference) (OtherComp :type Primitive%20Component%20Object%20Reference) (OtherBodyIndex :type Integer))
  (Utilities|Casting|CastToBP_FirstPersonCharacter OtherActor)
  (Rendering|SetVisibility (Variables|Default|GetWidget) false false))

(event EventBeginPlay
  (|CallParentFunction)
  (Variables|Default|SetEnemyHP 1e+02)
  (bind _asai_health_widget (Utilities|Casting|CastToAI_HealthWidget (UserInterface|GetUserWidgetObject (Variables|Default|GetWidget))))
  (Variables|Default|SetHealthWidgetREF_0 _asai_health_widget))

(event Game|Damage|EventAnyDamage
  (params (Damage :type Float%20%28single-precision%29) (DamageType :type Damage%20Type%20Object%20Reference) (InstigatedBy :type Controller%20Object%20Reference) (DamageCauser :type Actor%20Object%20Reference))
  (Variables|Default|Set현재%20체력 (Math|Float|Clamp(Float) (- (Variables|Default|Get현재%20체력) Damage) 0.0 (Variables|Default|Get최대%20체력))))

(fn ConstructionScript
  (|CallParentFunction))

(fn WeaponSetup
  (bind _weapon (Variables|Default|GetWeapon))
  (bind _weapon_2 (Variables|Default|GetWeapon))
  (bind _weapon_3 (Variables|Default|GetWeapon))
  (|CallParentFunction)
  (switch Utilities|FlowControl|Switch|SwitchonE_AI_WeaponType (Variables|Default|GetAIWeponTypes)
    (:NewEnumerator0
      ;[1 1 1] AssaultRifle
      (Transformation|SetWorldScale3D _weapon_3 "1.000000,1.000000,1.000000")
      (Transformation|SetRelativeLocationAndRotation _weapon_3 "-2.000000,-28.000000,-4.000000" "0, 0, 0" false false)
      (Class|SkinnedMeshComponent|SetSkeletalMesh _weapon_3 "/Game/ShooterAI/Weapons/AssaultRifle/Mesh/AssaultRifle.AssaultRifle" true)
      (Variables|Default|SetWeaponSound "/Game/ShooterAI/Audio/SC_WeaponFire_Cue.SC_WeaponFire_Cue")
      (Variables|Default|SetWeaponFireRate 0.5)
      (Variables|Default|SetWeaponDamage 3.0)
      (bind _output_get (Variables|Default|SetMaxAmmo 10))
      (Variables|Default|SetAmmoInMag _output_get)
      (Variables|Default|SetWeaponRecoil 1e+01)
      (Variables|Default|SetWeaponAimTime 0.3)
      (Variables|Default|SetReloadAnimPlayRate 1.0)
      (Variables|Default|SetWeaponReloadMontage "/Game/ShooterAI/Animations/AM_Reload_Rifle_Ironsights.AM_Reload_Rifle_Ironsights"))
    (:NewEnumerator1
      ;[1 1 1] Machine Gun
      (Transformation|SetWorldScale3D _weapon_2 "1.000000,1.000000,1.000000")
      (Transformation|SetRelativeLocationAndRotation _weapon_2 "-0.900000,15.000000,11.000000" "0,-2.000000, 0" false false)
      (Class|SkinnedMeshComponent|SetSkeletalMesh _weapon_2 "/Game/ShooterAI/Weapons/MachineGun/Mesh/SM_MachineGun.SM_MachineGun" true)
      (Variables|Default|SetWeaponSound "/Game/ShooterAI/Audio/SC_WeaponFire_Cue.SC_WeaponFire_Cue")
      (Variables|Default|SetWeaponFireRate 0.2)
      (Variables|Default|SetWeaponDamage 1e+01)
      (bind _output_get_2 (Variables|Default|SetMaxAmmo 15))
      (Variables|Default|SetAmmoInMag _output_get_2)
      (Variables|Default|SetWeaponRecoil 2e+01)
      (Variables|Default|SetWeaponAimTime 0.5)
      (Variables|Default|SetReloadAnimPlayRate 0.8)
      (Variables|Default|SetWeaponReloadMontage "/Game/ShooterAI/Animations/AM_Reload_Rifle_Ironsights.AM_Reload_Rifle_Ironsights"))
    (:NewEnumerator2
      ;[1 1 1] Sniper Rifle
      (Transformation|SetWorldScale3D _weapon "0.110000,0.110000,0.110000")
      (Transformation|SetRelativeLocationAndRotation _weapon "-0.907428,3.833228,-7.000000" "0,94.000000, 0" false false)
      (Class|SkinnedMeshComponent|SetSkeletalMesh _weapon "/Game/ShooterAI/Weapons/SniperRifle/Mesh/SM_SniperRifle.SM_SniperRifle" true)
      (Variables|Default|SetWeaponSound "/Game/ShooterAI/Audio/SC_WeaponFire_Cue.SC_WeaponFire_Cue")
      (Variables|Default|SetWeaponFireRate 3.0)
      (Variables|Default|SetWeaponDamage 15.0)
      (bind _output_get_3 (Variables|Default|SetMaxAmmo 1))
      (Variables|Default|SetAmmoInMag _output_get_3)
      (Variables|Default|SetWeaponRecoil 5.0)
      (Variables|Default|SetWeaponAimTime 1.0)
      (Variables|Default|SetReloadAnimPlayRate 0.8)
      (Variables|Default|SetWeaponReloadMontage "/Game/ShooterAI/Animations/AM_Reload_Rifle_Ironsights.AM_Reload_Rifle_Ironsights"))))