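; BP_Enemy_AICannon is the AI logic for an enemy cannon siege unit, running BT_Enemy_AICannon on BeginPlay.
; AI Perception updates pass each updated actor to CheckActor, which only handles actors tagged FRIEND.
; CheckActor toggles the blackboard's ActorKey: it stores the actor when the key is empty and clears it when already set.
; A FRIEND-tag actor search also runs per update, but its result is unused.
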(event OnPerceptionUpdated(AIPerception)
  (params (UpdatedActors :type Array%20of%20Actor%20Object%20References))
  (for _array_element UpdatedActors
    (Actor|GetAllActorswithTag "FRIEND")
    (CallFunction|CheckActor _array_element)))

(event EventBeginPlay
  (AI|RunBehaviorTree "/Game/공성유닛/Enemy_AI/BT_Enemy_AICannon.BT_Enemy_AICannon"))

(event EventTick
  (params (DeltaSeconds :type Float%20%28single-precision%29)))

(fn ConstructionScript)

(fn CheckActor
  (params (SensedActor :type Actor%20Object%20Reference))
  (if (Actor|ActorHasTag SensedActor "FRIEND")
    (Utilities|IsValid (AI|Components|Blackboard|GetValueasObject (AI|GetBlackboard 0) (Utilities|Name|MakeLiteralName "ActorKey"))
      (:Is%20Valid
        (AI|Components|Blackboard|SetValueasObject (AI|GetBlackboard 0) (Utilities|Name|MakeLiteralName "ActorKey") 0))
      (:Is%20Not%20Valid
        (AI|Components|Blackboard|SetValueasObject (AI|GetBlackboard 0) (Utilities|Name|MakeLiteralName "ActorKey") SensedActor)))))