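; BP_Friend_공성유닛 is a siege unit that fires cannonballs toward the player character's position.
; Fire rotates the actor to face player 0, plays explosion effects and sound, then spawns a scaled-down BP_대포알 at the 발사방향 component's location and rotation.
; SetMode stores a mode but its switch branches are empty, and the event graph is unused, so Fire relies on an external caller.
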(event EventBeginPlay)

(event Collision|EventActorBeginOverlap
  (params (OtherActor :type Actor%20Object%20Reference)))

(event EventTick
  (params (DeltaSeconds :type Float%20%28single-precision%29)))

(fn ConstructionScript)

(fn SetMode
  (params (Mode :type Integer))
  (bind _output_get (Variables|Default|SetMode Mode))
  (switch int _output_get))

(fn Fire
  (Transformation|SetActorRotation (Math|Rotator|FindLookatRotation (Transformation|GetActorLocation) (Transformation|GetActorLocation (Game|GetPlayerCharacter 0))))
  (Effects|SpawnEmitteratLocation "/Game/StarterContent/Particles/P_Explosion.P_Explosion" (Transformation|GetActorLocation) "0, 0, 0" "3.000000,3.000000,3.000000")
  (Audio|PlaySoundatLocation "/Game/StarterContent/Audio/Explosion02.Explosion02" "0, 0, 0" "0, 0, 0" 1.0 1.0 0.0 0 0 0 0)
  (Game|SpawnActorfromClass "/Game/공성유닛/BP_대포알.BP_대포알_C" (Math|Transform|MakeTransform (Transformation|GetWorldLocation (Variables|Default|Get발사방향)) (Transformation|GetWorldRotation (Variables|Default|Get발사방향)) "0.300000,0.300000,0.300000") "AdjustIfPossibleButAlwaysSpawn" 0 0))