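; Friendly siege unit with health, a proximity-shown health widget and a cannon attack.
; Damage lowers clamped health, updates the widget and destroys the unit at zero; the widget shows while the first-person character is inside the sphere.
; Fire, not called here, faces the nearest sphere-overlapping actor, unfiltered, then spawns explosion effects and a cannonball from the 발사방향 component.
; SetMode only stores the mode, with an empty switch.
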(event OnComponentBeginOverlap(Sphere)
  (params (OverlappedComponent :type Primitive%20Component%20Object%20Reference) (OtherActor :type Actor%20Object%20Reference) (OtherComp :type Primitive%20Component%20Object%20Reference) (OtherBodyIndex :type Integer) (bFromSweep :type Boolean) (SweepResult :type Hit%20Result%20Structure%20%28by%20ref%29))
  (Utilities|Casting|CastToBP_FirstPersonCharacter OtherActor)
  (Rendering|SetVisibility (Variables|Default|GetWidget) true false))

(event OnComponentEndOverlap(Sphere)
  (params (OverlappedComponent :type Primitive%20Component%20Object%20Reference) (OtherActor :type Actor%20Object%20Reference) (OtherComp :type Primitive%20Component%20Object%20Reference) (OtherBodyIndex :type Integer))
  (Utilities|Casting|CastToBP_FirstPersonCharacter OtherActor)
  (Rendering|SetVisibility (Variables|Default|GetWidget) false false))

(event EventBeginPlay
  (Variables|Default|SetHealth (Variables|Default|GetMaxHealth))
  (bind _asai_health_widget (Utilities|Casting|CastToAI_HealthWidget (UserInterface|GetUserWidgetObject (Variables|Default|GetWidget))))
  (Variables|Default|SetHealthWidgetREF _asai_health_widget))

(event Game|Damage|EventAnyDamage
  (params (Damage :type Float%20%28single-precision%29) (DamageType :type Damage%20Type%20Object%20Reference) (InstigatedBy :type Controller%20Object%20Reference) (DamageCauser :type Actor%20Object%20Reference))
  (bind _output_get (Variables|Default|SetHealth (Math|Float|Clamp(Float) (- (Variables|Default|GetHealth) Damage) 0.0 (Variables|Default|GetMaxHealth))))
  (Variables|/Game/widgets/AI_HealthWidget.AI_HealthWidget_C|SetHealth (Variables|Default|GetHealthWidgetREF) _output_get)
  (if (== (Variables|Default|GetHealth) 0.0)
    (Actor|DestroyActor)))

(fn ConstructionScript)

(fn SetMode
  (params (Mode :type Integer))
  (bind _output_get (Variables|Default|SetMode Mode))
  (switch int _output_get))

(fn Fire
  (Transformation|SetActorRotation (Math|Rotator|FindLookatRotation (Transformation|GetActorLocation) (Transformation|GetActorLocation (.ReturnValue (Actor|FindNearestActor (Transformation|GetActorLocation self) (Collision|GetOverlappingActors (Variables|Default|GetSphere) 0 :!class /Script/Engine.PrimitiveComponent))))))
  (Effects|SpawnEmitteratLocation "/Game/StarterContent/Particles/P_Explosion.P_Explosion" (Transformation|GetActorLocation) "0, 0, 0" "3.000000,3.000000,3.000000")
  (Audio|PlaySoundatLocation "/Game/StarterContent/Audio/Explosion02.Explosion02" "0, 0, 0" "0, 0, 0" 1.0 1.0 0.0 0 0 0 0)
  (Game|SpawnActorfromClass "/Game/공성유닛/BP_대포알.BP_대포알_C" (Math|Transform|MakeTransform (Transformation|GetWorldLocation (Variables|Default|Get발사방향)) (Transformation|GetWorldRotation (Variables|Default|Get발사방향)) "0.300000,0.300000,0.300000") "AdjustIfPossibleButAlwaysSpawn" 0 0))